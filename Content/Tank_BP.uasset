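; Tank Blueprint that wires up its turret and barrel and handles aim camera input.
; On BeginPlay it passes the TankTurret and TankBarrel components to setter functions defined outside these graphs.
; The AimAzimuth axis yaws an AzimuthGimbal and AimElevation pitches the SpringArm, splitting camera rotation across two components in local space.
; Axis values apply directly as rotation deltas, without delta-time scaling or pitch limits.
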(event `self.ReceiveBeginPlay`
  (`self.SetTurretReference` (`self.TankTurret`))
  (`self.SetBarrelReference` (`self.TankBarrel`)))

(event `InputAxis|AimAzimuth`
  (params (AxisValue :type "Float (single-precision)"))
  ;[1 1 1] Camera Input Binding
  (`SceneComponent.K2_AddLocalRotation` (`self.AzimuthGimbal`) (`KismetMathLibrary.MakeRotator` 0.0 0.0 AxisValue) false false))

(event `InputAxis|AimElevation`
  (params (AxisValue :type "Float (single-precision)"))
  ;[1 1 1] Camera Input Binding
  (`SceneComponent.K2_AddLocalRotation` (`self.SpringArm`) (`KismetMathLibrary.MakeRotator` 0.0 AxisValue) false false))

(fn `UserConstructionScript`)